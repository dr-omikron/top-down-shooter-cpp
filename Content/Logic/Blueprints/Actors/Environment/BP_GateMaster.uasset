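; BP_GateMaster is an automatic double-door gate that opens and closes around characters.
; Overlapping OpenTrigger opens it and leaving CloseTrigger closes it, with both filtering actors through GetCharacterRefMessage and playing sounds.
; On opening, each door's current relative location and an OpenDistance offset along X are captured as endpoints.
; StartTimer plays or reverses the Doors timeline, which lerps both doors between those endpoints.
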(event `self.OpenTrigger.OnComponentBeginOverlap`
  (params (OverlappedComponent :type "PrimitiveComponent Object Reference") (OtherActor :type "Actor Object Reference") (OtherComp :type "PrimitiveComponent Object Reference") (OtherBodyIndex :type Integer) (bFromSweep :type Boolean) (SweepResult :type "HitResult Structure (by ref)"))
  (bind (_relative_locationl_x _relative_locationl_y _relative_locationl_z) (`KismetMathLibrary.BreakVector` (`self.Relative LocationL`)))
  (bind (_relative_locationr_x _relative_locationr_y _relative_locationr_z) (`KismetMathLibrary.BreakVector` (`self.Relative LocationR`)))
  (bind _returnvalue (`SceneComponent.K2_GetComponentLocation` (`self.Gate`)))
  (bind _character (message `/Game/Logic/Blueprints/Interfaces/BPI_CharacterInterface.GetCharacterRef` OtherActor))
  (`/Engine/EditorBlueprintResources/StandardMacros.IsValid` _character
    (:`Is Valid`
      (if (not (`self.bDoorIsOpen`))
        (set `self.Relative LocationL` (`SceneComponent.RelativeLocation` (`self.GateDoorL`)))
        (set `self.Relative LocationR` (`SceneComponent.RelativeLocation` (`self.GateDoorR`)))
        (set `self.OpenLocationR` (`KismetMathLibrary.MakeVector` (- _relative_locationr_x (`self.OpenDistance`)) _relative_locationr_y _relative_locationr_z))
        (set `self.OpenLocationL` (`KismetMathLibrary.MakeVector` (+ _relative_locationl_x (`self.OpenDistance`)) _relative_locationl_y _relative_locationl_z))
        (set `self.bDoorIsOpen` true)
        (`self.StartTimer`)
        (`GameplayStatics.PlaySoundAtLocation` "/Game/Sounds/Environment/Pip1.Pip1" _returnvalue (struct) 1.0 1.0 0.0 null null null null)
        (`GameplayStatics.PlaySoundAtLocation` "/Game/Sounds/Environment/DoorOpen.DoorOpen" _returnvalue (struct) 1.0 1.0 0.0 null null null null)))))

(event `self.CloseTrigger.OnComponentEndOverlap`
  (params (OverlappedComponent :type "PrimitiveComponent Object Reference") (OtherActor :type "Actor Object Reference") (OtherComp :type "PrimitiveComponent Object Reference") (OtherBodyIndex :type Integer))
  (bind _character (message `/Game/Logic/Blueprints/Interfaces/BPI_CharacterInterface.GetCharacterRef` OtherActor))
  (`/Engine/EditorBlueprintResources/StandardMacros.IsValid` _character
    (:`Is Valid`
      (if (`self.bDoorIsOpen`)
        (set `self.bDoorIsOpen` false)
        (`self.StartTimer`)
        (`GameplayStatics.PlaySoundAtLocation` "/Game/Sounds/Environment/DoorOpen.DoorOpen" (`SceneComponent.K2_GetComponentLocation` (`self.Gate`)) (struct) 1.0 1.0 0.0 null null null null)))))

(event `StartTimer`
  (if (`self.bDoorIsOpen`)
    (bind (_direction _locationalpha) (`Timeline|Doors` :!label _label)
      (:`Update`
        (`SceneComponent.K2_SetRelativeLocation` (`self.GateDoorR`) (`KismetMathLibrary.VLerp` (`self.Relative LocationR`) (`self.OpenLocationR`) _locationalpha) false false)
        (`SceneComponent.K2_SetRelativeLocation` (`self.GateDoorL`) (`KismetMathLibrary.VLerp` (`self.Relative LocationL`) (`self.OpenLocationL`) _locationalpha) false false)))
    (else
      (goto _label :!via `Reverse`))))

(fn `UserConstructionScript`)
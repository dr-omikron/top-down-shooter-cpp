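; Player controller for a top-down character that slides the camera toward the cursor while aiming or walking.
; Each tick, SlideCamera steps the character's CameraBoom in XY toward a distant cursor up to a maximum offset, or interpolates it back when the cursor is near.
; Distance thresholds scale with boom arm length, tuning values come from the character, and the outward step ignores delta time.
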(event `self.ReceiveBeginPlay`
  (bind _character (message `/Game/Logic/Blueprints/Interfaces/BPI_CharacterInterface.GetCharacterRef` (`GameplayStatics.GetPlayerCharacter` 0)))
  (set `self.CharacterRef` _character))

(event `self.ReceiveTick`
  (params (DeltaSeconds :type "Float (single-precision)"))
  (`self.SlideCamera` DeltaSeconds))

(fn `SlideCamera`
  (params (DeltaTime :type "Float (double-precision)"))
  (locals (ClampedCameraHeight :type "Float (double-precision)" :default 0.0) (CameraLocation :type "Vector Structure" :default (0.0 0.0 0.0)) (CursorLocation :type "Vector Structure" :default (0.0 0.0 0.0)) (CharacterLocation :type "Vector Structure" :default (0.0 0.0 0.0)) (DistanceCharacterToCursor :type "Float (double-precision)" :default 0.0) (MaxClampedDistance :type "Float (double-precision)" :default 0.0) (MinClampedDistance :type "Float (double-precision)" :default 0.0) (DistanceChatacterToCamera :type "Float (double-precision)" :default 0.0) (SlideCamMuliplayer :type "Float (double-precision)" :default 0.0) (DeltaTimeLocal :type "Float (double-precision)"))
  (bind _characterref (`self.CharacterRef`))
  (bind _characterref_2 (`self.CharacterRef`))
  (bind _characterref_3 (`self.CharacterRef`))
  (bind _characterref_4 (`self.CharacterRef`))
  (bind (_x _y _z) (`KismetMathLibrary.BreakVector3f` (`local.CameraLocation`)))
  (bind _cameraboom (`TDSCharacter.CameraBoom` _characterref_4))
  (bind _movementstate (`StaminaComponentBase.MovementState` (`TDSCharacter.StaminaComponent` _characterref_3)))
  (bind (_x_2 _y_2) (`KismetMathLibrary.BreakVector2D` (* (`KismetMathLibrary.Normal2D` (`KismetMathLibrary.Conv_VectorToVector2D` (`KismetMathLibrary.GetForwardVector` (`KismetMathLibrary.FindLookAtRotation` (`local.CharacterLocation`) (`local.CursorLocation`))))) (`local.SlideCamMuliplayer`))))
  (set `local.DeltaTimeLocal` DeltaTime)
  (set `local.CursorLocation` (`self.GetCursorLocation`))
  (set `local.CameraLocation` (`SceneComponent.K2_GetComponentLocation` _cameraboom))
  (set `local.CharacterLocation` (`SceneComponent.K2_GetComponentLocation` (`Character.CapsuleComponent` _characterref_4)))
  (set `local.ClampedCameraHeight` (`KismetMathLibrary.MapRangeClamped` (`SpringArmComponent.TargetArmLength` _cameraboom) (`/Game/Logic/Blueprints/Character/Blueprints/BP_TopDownCharacter.MinCameraHeight` _characterref) (`/Game/Logic/Blueprints/Character/Blueprints/BP_TopDownCharacter.MaxCameraHeight` _characterref) 0.5 1.0))
  (set `local.DistanceCharacterToCursor` (`KismetMathLibrary.VSize` (- (`local.CursorLocation`) (`local.CharacterLocation`))))
  (set `local.DistanceChatacterToCamera` (`KismetMathLibrary.VSize2D` (`KismetMathLibrary.Conv_VectorToVector2D` (- (`local.CameraLocation`) (`local.CharacterLocation`)))))
  (set `local.MaxClampedDistance` (`/Game/Logic/Blueprints/Character/Blueprints/BP_TopDownCharacter.MaxDistanceSlideCam` _characterref_3))
  (set `local.MinClampedDistance` (`/Game/Logic/Blueprints/Character/Blueprints/BP_TopDownCharacter.MinDistanceSlideCam` _characterref_3))
  (set `local.SlideCamMuliplayer` (`/Game/Logic/Blueprints/Character/Blueprints/BP_TopDownCharacter.SpeedSlideCam` _characterref_3))
  (if (or (`|EnumEquality` _movementstate "Aim_State") (`|EnumEquality` _movementstate "Walk_State"))
    (if (> (`local.DistanceCharacterToCursor`) (* (`local.ClampedCameraHeight`) (`local.MinClampedDistance`)))
      (if (not (> (`local.DistanceChatacterToCamera`) (* (`local.ClampedCameraHeight`) (`local.MaxClampedDistance`))))
        (`SceneComponent.K2_SetWorldLocation` (`TDSCharacter.CameraBoom` (`self.CharacterRef`)) (`KismetMathLibrary.MakeVector` (+ _x_2 _x) (+ _y_2 _y) _z) false false))
      (else
        (`SceneComponent.K2_SetWorldLocation` (`TDSCharacter.CameraBoom` _characterref_2) (`KismetMathLibrary.VInterpTo` (`local.CameraLocation`) (`local.CharacterLocation`) (`local.DeltaTimeLocal`) (`/Game/Logic/Blueprints/Character/Blueprints/BP_TopDownCharacter.InterpolationSpeedSlideCam` _characterref_2)) false false)))))

(fn `UserConstructionScript`)